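; BP_Dome is a procedural mesh Blueprint that builds a sphere with a hole cut out of it.
; The Construction Script uses Geometry Script to reset the dynamic mesh and append a static sphere mesh scaled by SphereScale.
; It then boolean-subtracts a second sphere mesh placed by HoleTransform, using compute meshes as intermediates.
; All work happens at construction, as the event graph has no active logic.
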(event EventBeginPlay)

(event Collision|EventActorBeginOverlap
  (params (OtherActor :type Actor%20Object%20Reference)))

(event EventTick
  (params (DeltaSeconds :type Float%20%28single-precision%29)))

(fn ConstructionScript
  (bind _returnvalue (DynamicMeshComponent|GetDynamicMesh (Variables|DynamicMeshActor|GetDynamicMeshComponent)))
  (DynamicMesh|Reset _returnvalue)
  (bind _returnvalue_2 (DynamicMeshActor|AllocateComputeMesh))
  (bind _returnvalue_3 (GeometryScript|StaticMesh|CopyMeshFromStaticMesh :FromStaticMeshAsset "/Game/01Models/Sphere.Sphere" :ToDynamicMesh _returnvalue_2 :Debug 0)
    (:Success
      (bind _returnvalue_4 (DynamicMeshComponent|GetDynamicMesh (Variables|DynamicMeshActor|GetDynamicMeshComponent)))
      (bind _returnvalue_5 (GeometryScript|MeshEdits|AppendMesh _returnvalue_4 _returnvalue_3 (Math|Transform|MakeTransform "0, 0, 0" "0, 0, 0" (Variables|Default|GetSphere%20Scale)) false "(CombineMode=EnableAllMatching)" 0))
      (bind _returnvalue_6 (DynamicMeshActor|AllocateComputeMesh))
      (bind _returnvalue_7 (GeometryScript|StaticMesh|CopyMeshFromStaticMesh :FromStaticMeshAsset "/Engine/EditorMeshes/ArcadeEditorSphere.ArcadeEditorSphere" :ToDynamicMesh _returnvalue_6 :Debug 0)
        (:Success
          (GeometryScript|Booleans|ApplyMeshBoolean :TargetMesh _returnvalue_5 :ToolMesh _returnvalue_7 :ToolTransform (Variables|Default|GetHole%20Transform) :Operation "Subtract" :Debug 0))))))